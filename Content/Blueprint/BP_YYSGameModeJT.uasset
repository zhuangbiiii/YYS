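; BP_YYSGameModeJT is a game mode that relays player login and logout to other objects through interface messages.
; On PostLogin it sends a login message to the new player controller, flagging whether its controller ID is zero.
; On logout it passes the exiting controller to the game state.
; A debug print of login name and player count is left disconnected.
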(event EventPostLogin
  (params (NewPlayer :type Player%20Controller%20Object%20Reference))
  (Class|BPIServerGameStage|IonPlayerLogin(Message) NewPlayer (== (Class|GameplayStatics|GetPlayerControllerID NewPlayer) 0)))

(event EventOnLogout
  (params (ExitingController :type Controller%20Object%20Reference))
  (Class|BPIServerGameStage|IonPlayerLogout(Message) (Game|GetGameState) ExitingController))

(fn ConstructionScript)
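; BP_YYSPlayerState is a PlayerState that tracks a player's ready and homeowner (session owner) flags and relays pre-game messages.
; Interface events trigger custom RPC events: the server one stores readiness and notifies the GameState.
; Client ones forward login and game-ready messages to player controller 0 through interface calls.
; The game-start handler is empty, and some disconnected debug prints remain.
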(event Custom|E_SERVER:OnPlayerReady
  (params (isReady :type Boolean))
  (Class|YYSPlayerState|SetPlayerReady isReady)
  (Class|BPIYYSInterface|IonPlayerReady(Message) (Game|GetGameState) false))

(event Custom|E_CLIENT:OnPlayerLogin
  (Class|BPIYYSInterface|IonPlayerLogin(Message) (Game|GetPlayerController 0) false))

(event Custom|E_CLIENT:OnGameReady
  (bind _returnvalue (Game|GetPlayerController 0))
  (Development|PrintString (Utilities|GetDisplayName _returnvalue))
  (Class|BPIYYSInterface|IonGameReady(Message) _returnvalue))

(event EventIonPlayerReady
  (params (isReady? :type Boolean))
  (CallFunction|ESERVER:OnPlayerReady isReady?))

(event EventIonGameStart)

(event EventIonGameReady
  (CallFunction|ECLIENT:OnGameReady))

(event EventIonPlayerLogin
  (params (isSessionOwner? :type Boolean))
  (Class|YYSPlayerState|SetHomeowner isSessionOwner?)
  (CallFunction|ECLIENT:OnPlayerLogin))

(fn ConstructionScript)
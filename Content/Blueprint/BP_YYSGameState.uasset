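; Game state Blueprint that starts the match once every player has readied up.
; OnPlayerReady forwards to a server event, which runs a check over PlayerArray for each BP_YYSPlayerState's ready flag.
; When all are ready it calls OnGameStartMessage on player controller 0; otherwise it prints a not-ready message.
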(event Custom|Server:OnPlayerReady
  (bind _state (CallFunction|FIsAllPlayerReady))
  (if _state
    (Class|BPIGameStage|OnGameStart(Message) (Game|GetPlayerController 0))
    (else
      (Development|PrintString "Some player not ready yet."))))

(event EventOnPlayerReady
  (CallFunction|Server:OnPlayerReady))

(fn ConstructionScript)

(fn FIsAllPlayerReady
  (for _array_element (Variables|Default|GetPlayerArray)
    (bind _asbp_yysplayer_state (Utilities|Casting|CastToBP_YYSPlayerState _array_element))
    (if (not (Class|YYSPlayerState|IsPlayerReady _asbp_yysplayer_state))
      (return (Class|YYSPlayerState|IsPlayerReady _asbp_yysplayer_state))))
  (return true))